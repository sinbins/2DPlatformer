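; Paper2D player character Blueprint with side-scrolling run and jump via Enhanced Input, adding its mapping context on BeginPlay.
; Movement input drives the character along world X, swaps run and idle flipbooks, and rotates the sprite to face the travel direction.
; Jumping plays a non-looping flipbook and blocks movement input until a short-delay polling loop sees zero vertical velocity, then restores looping idle.
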(event Input|EnhancedActionEvents|EnhancedInputActionIA_Movement
  (params (ActionValue :type Float%20%28double-precision%29) (ElapsedSeconds :type Float%20%28double-precision%29) (TriggeredSeconds :type Float%20%28double-precision%29) (InputAction :type Input%20Action%20Object%20Reference :default "/Game/Assets/BluePrints/IA_Movement.IA_Movement"))
  (:Triggered
    (if (not (Variables|Default|GetisJumping))
      (Pawn|Input|AddMovementInput (Math|Vector|GetForwardVector "0, 0, 0") ActionValue false)
      (Sprite|SetFlipbook (Variables|Default|GetSprite) "/Game/Assets/Flipbooks/FB_Run.FB_Run")
      (if (> ActionValue 0.0)
        (Transformation|SetWorldRotation (Variables|Default|GetSprite) "0, 0, 0" false false)
        (else
          (Transformation|SetWorldRotation (Variables|Default|GetSprite) "0.000000,-180.000000,0.000000" false false)))))
  (:Completed
    (if (not (Variables|Default|GetisJumping))
      (Sprite|SetFlipbook (Variables|Default|GetSprite) "/Game/Assets/Flipbooks/FB_Idle.FB_Idle"))))

(event Input|EnhancedActionEvents|EnhancedInputActionIA_Jump
  (params (ActionValue :type Boolean) (ElapsedSeconds :type Float%20%28double-precision%29) (TriggeredSeconds :type Float%20%28double-precision%29) (InputAction :type Input%20Action%20Object%20Reference :default "/Game/Assets/BluePrints/IA_Jump.IA_Jump"))
  (bind _sprite (Variables|Default|GetSprite))
  (:Triggered
    (if (not (Variables|Default|GetisJumping))
      (Variables|Default|SetisJumping true)
      (Character|Jump)
      (Components|Timeline|SetLooping _sprite false)
      (Sprite|SetFlipbook _sprite "/Game/Assets/Flipbooks/FB_Jump.FB_Jump")
      (Utilities|FlowControl|Delay 0.1)
      (if (== (.Z (Math|Vector|BreakVector (Transformation|GetVelocity))) 0.0) :!label _label
        (Components|Timeline|SetLooping _sprite true)
        (Audio|Components|Audio|Play _sprite)
        (Sprite|SetFlipbook _sprite "/Game/Assets/Flipbooks/FB_Idle.FB_Idle")
        (Variables|Default|SetisJumping false)
        (else
          (Utilities|FlowControl|Delay 0.1)
          (goto _label))))))

(event EventBeginPlay
  (bind _asbp_player_controller (Utilities|Casting|CastTobp_playerController (Pawn|GetController)))
  (Input|AddMappingContext (PlayerController|LocalPlayerSubsystems|GetEnhancedInputLocalPlayerSubsystem _asbp_player_controller) "/Game/Assets/BluePrints/IMC_Default.IMC_Default" 0 "(bIgnoreAllPressedKeysUntilRelease=True,bForceImmediately=False,bNotifyUserSettings=False)"))

(fn ConstructionScript)